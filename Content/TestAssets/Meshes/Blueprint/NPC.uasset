(event `Patrol`
  (params (first_point :type "/Game/TestAssets/Meshes/Blueprint/PatrolPoint Object Reference"))
  (bind _next_point (`/Game/TestAssets/Meshes/Blueprint/PatrolPoint.next_point` first_point))
  ;[1 1 1] Patrol
  (`|AIMoveTo` first_point self (0.0 0.0 0.0) first_point
    (:`OnSuccess`
      (`KismetSystemLibrary.Delay` (`/Game/TestAssets/Meshes/Blueprint/PatrolPoint.duration` first_point))
      (`/Engine/EditorBlueprintResources/StandardMacros.IsValid` _next_point
        (:`Is Valid`
          (`self.Patrol` self _next_point))))))

(event `self.PawnSensing.OnSeePawn`
  (params (Pawn :type "Pawn Object Reference"))
  ;[1 1 1] Follow on sigth
  (bind _asfirst_person_character_no_gun (cast `/Game/TestAssets/Meshes/Blueprint/FirstPersonCharacterNoGun` Pawn))
  (`|AIMoveTo` self (0.0 0.0 0.0) _asfirst_person_character_no_gun
    (:`then`
      (`KismetSystemLibrary.PrintString` "JE TE VOIS"))))

(fn `UserConstructionScript`)