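; House door Blueprint that the player can open and close with the Use input while standing inside its trigger volume.
; UseTrigger overlaps from FirstPersonCharacter or FirstPersonCharacterNoGun open and close a Gate node that filters the input.
; When a press passes the gate, a Locked door prints a French "locked" message; otherwise it toggles on the Openned flag, playing its ActorSequence forward or in reverse.
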(event `Open`
  ;[1 1 1] Open
  (`MovieSceneSequencePlayer.Play` (`ActorSequenceComponent.SequencePlayer` (`self.ActorSequence`)))
  (set `self.openned` true))

(event `Close`
  ;[1 1 1] Open
  (`MovieSceneSequencePlayer.PlayReverse` (`ActorSequenceComponent.SequencePlayer` (`self.ActorSequence`)))
  (set `self.openned` false))

(event `InputAction|Use` :consume false
  (params (Key :type "Key Structure"))
  ;[1 1 1] Gestion interaction
  (:`Pressed`
    (`/Engine/EditorBlueprintResources/StandardMacros.Gate` true :!label _label
      (:`Exit`
        (if (`self.locked`)
          (`KismetSystemLibrary.PrintString` "Porte verrouillée")
          (elif (`self.openned`)
            (`self.Close`)
            (else
              (`self.Open`))))))))

(event `self.UseTrigger.OnComponentBeginOverlap`
  (params (OverlappedComponent :type "PrimitiveComponent Object Reference") (OtherActor :type "Actor Object Reference") (OtherComp :type "PrimitiveComponent Object Reference") (OtherBodyIndex :type Integer) (bFromSweep :type Boolean) (SweepResult :type "HitResult Structure (by ref)"))
  ;[1 1 1] Gestion interaction
  (cast `/Game/TestAssets/Meshes/Blueprint/FirstPersonCharacterNoGun` OtherActor
    (:`then`
      (goto _label :!via `Open`))
    (:`CastFailed`
      (cast `/Game/FirstPersonBP/Blueprints/FirstPersonCharacter` OtherActor)
      (goto _label :!via `Open`))))

(event `self.UseTrigger.OnComponentEndOverlap`
  (params (OverlappedComponent :type "PrimitiveComponent Object Reference") (OtherActor :type "Actor Object Reference") (OtherComp :type "PrimitiveComponent Object Reference") (OtherBodyIndex :type Integer))
  ;[1 1 1] Gestion interaction
  (cast `/Game/TestAssets/Meshes/Blueprint/FirstPersonCharacterNoGun` OtherActor
    (:`then`
      (goto _label :!via `Close`))
    (:`CastFailed`
      (cast `/Game/FirstPersonBP/Blueprints/FirstPersonCharacter` OtherActor)
      (goto _label :!via `Close`))))

(fn `UserConstructionScript`)